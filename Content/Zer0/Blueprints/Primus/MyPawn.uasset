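; Pawn for a physics-driven hovering ship, steered by forward and right input axes on Tick.
; A downward sphere trace against static world objects records ground distance and normal, which the next tick's spring-like force uses to hold hover height.
; The same force adds input thrust along the mesh's forward and right vectors, while right input also applies yaw torque.
; Debug output prints the force and draws the ground normal.
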(event `self.ReceiveTick`
  (params (DeltaSeconds :type "Float (single-precision)"))
  (bind _returnvalue (`self.GetInputAxisValue`))
  (bind _returnvalue_2 (`SceneComponent.K2_GetComponentLocation` (`self.ShipMeshComponent`)))
  (bind _returnvalue_3 (* (+ (* (`SceneComponent.GetForwardVector` (`self.ShipMeshComponent`)) (`self.GetInputAxisValue`)) (* (`SceneComponent.GetRightVector` (`self.ShipMeshComponent`)) _returnvalue)) (* DeltaSeconds (`self.MovementSpeed`))))
  (bind _returnvalue_4 (+ (* (`self.GroundNormal`) (* (- (`self.DistanceToGround`) 60.0) -1000.0)) (* _returnvalue_3 5000.0)))
  (`|ExecutionSequence`
    (:`then_0`
      (if (> (`KismetMathLibrary.VSize` _returnvalue_3) 0.0)
        (`PrimitiveComponent.AddTorque` (`self.ShipMeshComponent`) (* (+ (`KismetMathLibrary.MakeVector` 0.0 0.0 _returnvalue) (0.0 0.0 0.0)) 10.0) "None" true)))
    (:`then_1`
      (`PrimitiveComponent.AddForce` (`self.ShipMeshComponent`) _returnvalue_4 "None" false)
      (`KismetSystemLibrary.PrintString` (`KismetStringLibrary.Conv_VectorToString` _returnvalue_4)))
    (:`then_2`
      (bind _outhit (`KismetSystemLibrary.SphereTraceSingleForObjects` _returnvalue_2 (+ _returnvalue_2 (0.0 0.0 -400.0)) 50.0 (`|MakeArray` "ObjectTypeQuery1" :!type "EObjectTypeQuery Enum")))
      (bind (_bblockinghit _binitialoverlap _time _location _impactpoint _normal) (`GameplayStatics.BreakHitResult` _outhit))
      (set `self.DistanceToGround` (`KismetMathLibrary.VSize` (- _returnvalue_2 _location)))
      (`KismetSystemLibrary.DrawDebugArrow` _location (+ _location (* _normal 50.0)) 50.0 (struct :`G` 0.089381 :`B` 0.99 :`A` 1.0))
      (set `self.GroundNormal` _normal))))

(fn `UserConstructionScript`)