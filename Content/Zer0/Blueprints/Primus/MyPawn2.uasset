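; Physics-driven hovering ship pawn with thrust, banked turning and a held boost, applied as forces and torques on the ship mesh.
; Each tick, four sphere traces (front, back, left, right) estimate ground slope and distance.
; The slope drives pitch and roll alignment, while distance drives a spring-like hover force, gravity toggling and a minimum-height teleport correction.
; Mesh hits spawn an explosion sound and particle effect.
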(event `self.ShipMeshComponent.OnComponentHit`
  (params (OtherActor :type "Actor Object Reference") (OtherComp :type "PrimitiveComponent Object Reference") (NormalImpulse :type "Vector Structure") (Hit :type "HitResult Structure (by ref)"))
  (bind _returnvalue (`SceneComponent.K2_GetComponentLocation` (`self.ShipMeshComponent`)))
  ;[1 1 1] Comment
  (bind _returnvalue_2 (`GameplayStatics.SpawnSoundAtLocation` "/Game/StarterContent/Audio/Explosion02.Explosion02" _returnvalue))
  (set `self.Audio` _returnvalue_2)
  (`GameplayStatics.SpawnEmitterAtLocation` "/Game/StarterContent/Particles/P_Explosion.P_Explosion" _returnvalue))

(event `self.ReceiveTick`
  (params (DeltaSeconds :type "Float (single-precision)"))
  (bind _mindistance (`self.MinDistance`))
  (bind _averagedistance (`self.AverageDistance`))
  (bind _returnvalue (`SceneComponent.K2_GetComponentRotation` (`self.ShipMeshComponent`)))
  (bind _returnvalue_2 (`SceneComponent.GetUpVector` (`self.ShipMeshComponent`)))
  (bind _returnvalue_3 (* (* DeltaSeconds (`self.GetInputAxisValue`)) (`self.TurnSpeed`)))
  (bind _returnvalue_4 (+ (`KismetMathLibrary.MakeVector` (.z (`KismetMathLibrary.LessLess_VectorRotator` (- (`self.ShipRoll`) (`self.GroundRoll`)) _returnvalue))) (`KismetMathLibrary.MakeVector` 0.0 (.z (`KismetMathLibrary.LessLess_VectorRotator` (- (`self.ShipPitch`) (`self.GroundPitch`)) _returnvalue)))))
  (`|ExecutionSequence`
    (:`then_0`
      ;[1 1 1] Handle User Input
      (`PrimitiveComponent.AddForce` (`self.ShipMeshComponent`) (* (* (* (`self.GetActorForwardVector`) (* (`self.GetInputAxisValue`) DeltaSeconds)) (+ (`self.MovementSpeed`) (* (`KismetMathLibrary.Conv_BoolToInt` (`self.isBoosting`)) (`self.Boost`)))) 10.0) "None" true)
      (`PrimitiveComponent.AddTorque` (`self.ShipMeshComponent`) (* (`KismetMathLibrary.GreaterGreater_VectorRotator` (`KismetMathLibrary.MakeVector` (* _returnvalue_3 -0.4) 0.0 _returnvalue_3) (`self.K2_GetActorRotation`)) 10.0) "None" true))
    (:`then_1`
      ;[1 1 1] Check for Ground
      (bind (_location _distance _hit) (`self.SphereTraceDown` (`self.FrontStart`)))
      (bind (_location_2 _distance_2 _hit_2) (`self.SphereTraceDown` (`self.BackStart`)))
      (if (and _hit _hit_2 (stale _hit_3) (stale _hit_4)) :!label _label
        (set `self.isFlying` false)
        (set `self.GroundPitch` (- _location _location_2))
        (set `self.GroundRoll` (- (stale _location_3) (stale _location_4)))
        (set `self.AverageDistance` (/ (+ _distance _distance_2 (stale _distance_3) (stale _distance_4)) 4.0))
        (else
          (set `self.GroundPitch` (* (`self.GroundRoll`) -1.0))
          (set `self.GroundRoll` (* (`self.GroundRoll`) -1.0))
          (set `self.AverageDistance` (+ (`self.MaxDistance`) 1.0))
          (set `self.isFlying` true))))
    (:`then_2`
      (bind (_location_3 _distance_3 _hit_3) (`self.SphereTraceDown` (`self.LeftStart`)))
      (bind (_location_4 _distance_4 _hit_4) (`self.SphereTraceDown` (`self.RightStart`)))
      (goto _label))
    (:`then_3`
      ;[1 1 1] Orient to Ground
      (set `self.ShipPitch` (- (`SceneComponent.K2_GetComponentLocation` (`self.FrontStart`)) (`SceneComponent.K2_GetComponentLocation` (`self.BackStart`))))
      (set `self.ShipRoll` (- (`SceneComponent.K2_GetComponentLocation` (`self.LeftStart`)) (`SceneComponent.K2_GetComponentLocation` (`self.RightStart`))))
      (if (not (`self.isFlying`))
        _
        (else
          _))
      (`PrimitiveComponent.AddTorque` (`self.ShipMeshComponent`) (* _returnvalue_4 5000.0) "None" false)
      (`PrimitiveComponent.SetPhysicsAngularVelocity` (`self.ShipMeshComponent`) (`KismetMathLibrary.GreaterGreater_VectorRotator` _returnvalue_4 _returnvalue) false "None"))
    (:`then_4`
      ;[1 1 1] Ground Offset
      (if (> _averagedistance _mindistance)
        (`PrimitiveComponent.SetEnableGravity` (`self.ShipMeshComponent`) (`self.isFlying`))
        (set `self.zAdd` (* (* _returnvalue_2 (- (`self.TargetDistance`) (`self.AverageDistance`))) 5000.0))
        (else
          (`SceneComponent.K2_AddWorldOffset` (`self.ShipMeshComponent`) (* _returnvalue_2 (- _mindistance _averagedistance)) false true)))
      (`PrimitiveComponent.AddForce` (`self.ShipMeshComponent`) (`self.zAdd`) "None" false))))

(event `InputAction|Boost`
  (params (Key :type "Key Structure" :default "AnyKey"))
  (:`Pressed`
    (set `self.isBoosting` true))
  (:`Released`
    (set `self.isBoosting` false)))

(fn `SphereTraceDown`
  (params (Start :type "SceneComponent Object Reference"))
  (returns (Location :type "Vector Structure") (Distance :type "Float (double-precision)") (Hit :type Boolean))
  (bind _returnvalue (`SceneComponent.K2_GetComponentLocation` Start))
  (bind (_outhit _returnvalue_2) (`KismetSystemLibrary.SphereTraceSingleForObjects` _returnvalue (+ _returnvalue (* (`SceneComponent.GetForwardVector` Start) 2000.0)) 50.0 (`|MakeArray` "ObjectTypeQuery1" :!type "EObjectTypeQuery Enum") true))
  (bind (_bblockinghit _binitialoverlap _time _location) (`GameplayStatics.BreakHitResult` _outhit))
  (return _location (`KismetMathLibrary.VSize` (- _returnvalue _location)) _returnvalue_2))

(fn `UserConstructionScript`)